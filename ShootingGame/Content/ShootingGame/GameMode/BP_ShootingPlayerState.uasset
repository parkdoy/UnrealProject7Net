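; Player state for the shooting game that holds each player's HP and Armor.
; AddDamage drains Armor first and passes any overflow to HP, while AddHeal and AddArmor raise their stats within fixed limits.
; RepNotify handlers for HP and Armor broadcast current and max values through event dispatchers.
; An older path that updated the name tag and HUD directly from the HP notify is left unconnected.
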(event `self.ReceiveBeginPlay`
  (`KismetSystemLibrary.PrintString` (`KismetStringLibrary.Concat_StrStr` "" (`KismetSystemLibrary.GetDisplayName` self))))

(fn `Add Damage`
  (params (Damage :type "Float (double-precision)"))
  (bind _returnvalue (- (`self.Armor`) Damage))
  (if (> _returnvalue 0.0)
    (set `self.Armor` (- (`self.Armor`) (`local.Damage`)))
    (else
      (set `self.Armor` 0.0)
      (bind _output_get (set `self.HP` (`KismetMathLibrary.FClamp` (+ _returnvalue (`self.HP`)) 0.0 100.0)))
      (`KismetSystemLibrary.PrintString` (`KismetStringLibrary.Concat_StrStr` "Add Damage Result : " (`KismetStringLibrary.Conv_DoubleToString` _output_get))))))

(fn `AddArmor`
  (params (Armor :type "Float (double-precision)"))
  (set `self.Armor` (`KismetMathLibrary.FClamp` (+ Armor (`self.Armor`)) 0.0 100.0)))

(fn `AddHeal`
  (params (Heal :type "Float (double-precision)"))
  (bind _output_get (set `self.HP` (`KismetMathLibrary.FClamp` (+ (`self.HP`) Heal) 0.0 100.0)))
  (`KismetSystemLibrary.PrintString` (`KismetStringLibrary.Conv_DoubleToString` _output_get)))

(fn `OnRep_Armor`
  (`self.EventDispatcher_Armor` (`self.Armor`) 100.0))

(fn `OnRep_HP`
  ;[1 1 1] Client
  (`KismetSystemLibrary.PrintString` (`KismetStringLibrary.Concat_StrStr` "OnRep_HP" (`KismetStringLibrary.Conv_DoubleToString` (`self.HP`))))
  (`self.EventDispatcher_HP` (`self.HP`) 100.0))

(fn `UserConstructionScript`)