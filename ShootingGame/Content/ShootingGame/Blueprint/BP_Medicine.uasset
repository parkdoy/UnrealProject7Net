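; BP_Medicine is a health pickup actor for the shooting game that heals a player character on touch.
; Its StaticMesh overlap runs only on the server, casts to BP_ShootingCharacter and its BP_ShootingPlayerState, calls AddHeal with a fixed amount, then destroys the actor.
; A disconnected hide, delay and re-show sequence remains in the graph but never runs, so the pickup is single-use.
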(event `self.StaticMesh.OnComponentBeginOverlap`
  (params (OverlappedComponent :type "PrimitiveComponent Object Reference") (OtherActor :type "Actor Object Reference") (OtherComp :type "PrimitiveComponent Object Reference") (OtherBodyIndex :type Integer) (bFromSweep :type Boolean) (SweepResult :type "HitResult Structure (by ref)"))
  (`/Engine/EditorBlueprintResources/ActorMacros.Switch Has Authority`
    (:`Authority`
      (bind _asbp_shooting_character (cast `/Game/ShootingGame/GameMode/BP_ShootingCharacter` OtherActor))
      (bind _asbp_shooting_player_state (cast `/Game/ShootingGame/GameMode/BP_ShootingPlayerState` (`Pawn.PlayerState` _asbp_shooting_character)))
      (`/Game/ShootingGame/GameMode/BP_ShootingPlayerState.AddHeal` _asbp_shooting_player_state (+ 0.0 50.0))
      (`self.K2_DestroyActor`))))

(fn `UserConstructionScript`)