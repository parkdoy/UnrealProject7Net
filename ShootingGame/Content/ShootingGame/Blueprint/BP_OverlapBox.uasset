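; BP_OverlapBox is a trigger cube in the shooting game that spawns a BP_Weapon at its own transform when something overlaps it.
; On overlap, only the authority hides the cube, disables its collision and spawns the weapon, with no filter on the overlapping actor.
; It then calls ReqBeginOverlap, a custom event that repeats the hide and collision disable.
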(event `self.ReceiveBeginPlay`)

(event `self.Cube.OnComponentBeginOverlap`
  (params (OverlappedComponent :type "PrimitiveComponent Object Reference") (OtherActor :type "Actor Object Reference") (OtherComp :type "PrimitiveComponent Object Reference") (OtherBodyIndex :type Integer) (bFromSweep :type Boolean) (SweepResult :type "HitResult Structure (by ref)"))
  (`/Engine/EditorBlueprintResources/ActorMacros.Switch Has Authority`
    (:`Authority`
      (`SceneComponent.SetVisibility` (`self.Cube`) false false)
      (`PrimitiveComponent.SetCollisionEnabled` (`self.Cube`) "NoCollision")
      (`|SpawnActorFromClass` "/Game/ShootingGame/Blueprint/BP_Weapon.BP_Weapon_C" (`self.GetTransform`) "Undefined" "OverrideRootScale" null null)
      (`self.ReqBeginOverlap`))))

(event `ReqBeginOverlap`
  (`SceneComponent.SetVisibility` (`self.Cube`) false false)
  (`PrimitiveComponent.SetCollisionEnabled` (`self.Cube`) "NoCollision"))

(fn `UserConstructionScript`)