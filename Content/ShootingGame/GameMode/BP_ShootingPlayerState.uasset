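; Player state for the shooting game, holding each player's HP, armor, name, kills and deaths.
; Damage drains armor first, but a hit that depletes it subtracts the full damage from HP because armor is zeroed before that calculation.
; RepNotify functions relay stat changes through event dispatchers.
; On BeginPlay it passes itself to the first player controller's BP_ShootingHud for binding, replacing disconnected direct nametag and HUD updates.
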(event `self.ReceiveBeginPlay`
  (`self.InitializeBind`))

(fn `Add Damage`
  (params (Damage :type "Float (double-precision)"))
  (bind _returnvalue (- (`self.Armor`) Damage))
  (if (> _returnvalue 0.0)
    (set `self.Armor` (- (`self.Armor`) (`local.Damage`)))
    (else
      (set `self.Armor` 0.0)
      (bind _output_get (set `self.HP` (`KismetMathLibrary.FClamp` (+ _returnvalue (`self.HP`)) 0.0 100.0)))
      (`KismetSystemLibrary.PrintString` (`KismetStringLibrary.Concat_StrStr` "Add Damage Result : " (`KismetStringLibrary.Conv_DoubleToString` _output_get)) false false))))

(fn `AddArmor`
  (params (Armor :type "Float (double-precision)"))
  (set `self.Armor` (`KismetMathLibrary.FClamp` (+ Armor (`self.Armor`)) 0.0 100.0)))

(fn `AddDeath`
  (set `self.Death` (+ (`self.Death`) 1)))

(fn `AddHeal`
  (params (Heal :type "Float (double-precision)"))
  (bind _output_get (set `self.HP` (`KismetMathLibrary.FClamp` (+ (`self.HP`) Heal) 0.0 100.0)))
  (`KismetSystemLibrary.PrintString` (`KismetStringLibrary.Conv_DoubleToString` _output_get)))

(fn `AddKill`
  (set `self.Kill` (+ (`self.Kill`) 1)))

(fn `InitializeBind`
  (bind _asbp_shooting_hud (cast `/Game/ShootingGame/GameMode/BP_ShootingHud` (`PlayerController.GetHUD` (`GameplayStatics.GetPlayerController` 0)))
    (:`then`
      (`/Game/ShootingGame/GameMode/BP_ShootingHud.Bind Player Stat` _asbp_shooting_hud self))
    (:`CastFailed`
      (`KismetSystemLibrary.PrintString` "BP_ShootingHUD Cast Failed" true true (struct :`R` 1.0 :`G` 0.014478 :`B` 0.102139 :`A` 1.0)))))

(fn `IsDeath`
  (returns (IsDeath :type Boolean))
  (return (<= (`self.HP`) 0.0)))

(fn `OnRep_Armor`
  (`self.EventDispatcher_Armor` (`self.Armor`) 100.0))

(fn `OnRep_Death`
  (`self.EventDispatcher_Death` (`self.Death`)))

(fn `OnRep_HP`
  ;[1 1 1] Client
  (`KismetSystemLibrary.PrintString` (`KismetStringLibrary.Concat_StrStr` "OnRep_HP" (`KismetStringLibrary.Conv_DoubleToString` (`self.HP`))) false false)
  (`self.EventDispatcher_HP` (`self.HP`) 100.0))

(fn `OnRep_Kill`
  (`self.EventDispatcher_Kill` (`self.Kill`)))

(fn `OnRep_Name`
  (`self.EventDispatcher_Name` (`self.Name`)))

(fn `SetName`
  (params (Name :type String))
  (set `self.Name` Name))

(fn `UserConstructionScript`)