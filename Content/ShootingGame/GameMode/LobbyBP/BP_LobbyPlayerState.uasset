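; BP_LobbyPlayerState is the lobby player state that holds a replicated Name for a player.
; On BeginPlay it registers itself with the first local player's BP_LobbyHUD through BindPlayerStates, printing an error if the cast fails.
; SetName writes the value, and its OnRep broadcasts a change-name event dispatcher so listeners can react to the new name.
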(event `self.ReceiveBeginPlay`
  (`self.Initialize Bind`))

(fn `Initialize Bind`
  (bind _asbp_lobby_hud (cast `/Game/ShootingGame/GameMode/LobbyBP/BP_LobbyHUD` (`PlayerController.GetHUD` (`GameplayStatics.GetPlayerController` 0)))
    (:`then`
      (`/Game/ShootingGame/GameMode/LobbyBP/BP_LobbyHUD.BindPlayerStates` _asbp_lobby_hud self))
    (:`CastFailed`
      (`KismetSystemLibrary.PrintString` "BP_LobbyHUD Cast Failed" true true (struct :`R` 1.0 :`G` 0.014478 :`B` 0.102139 :`A` 1.0)))))

(fn `OnRep_Name`
  (`self.NewEventDispatcher_ChangeName` (`self.Name`)))

(fn `SetName`
  (params (Name :type String))
  (set `self.Name` Name))

(fn `UserConstructionScript`)