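; Lobby player controller that hands the player's name from the game instance to their lobby player state.
; On possess, ResClientPossess reads Name from ShootingGameInstance and passes it to ReqSetNewName, which calls SetName on BP_LobbyPlayerState.
; The Res/Req event naming suggests a client-to-server round trip, though replication settings are not shown.
; BeginPlay and Tick are empty, and a possess debug print is left disconnected.
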(event `self.ReceivePossess`
  (params (PossessedPawn :type "Pawn Object Reference"))
  (`self.ResClientPossess`))

(event `ResClientPossess`
  (bind _asshooting_game_instance (cast `/Game/ShootingGame/GameMode/ShootingGameInstance` (`GameplayStatics.GetGameInstance`)))
  (`self.ReqSetNewName` (`/Game/ShootingGame/GameMode/ShootingGameInstance.Name` _asshooting_game_instance)))

(event `ReqSetNewName`
  (params (NewName :type String))
  (bind _asbp_lobby_player_state (cast `/Game/ShootingGame/GameMode/LobbyBP/BP_LobbyPlayerState` (`self.PlayerState`)))
  (`/Game/ShootingGame/GameMode/LobbyBP/BP_LobbyPlayerState.SetName` _asbp_lobby_player_state NewName))

(fn `UserConstructionScript`)