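; Lobby HUD that shows the lobby widget and keeps its player list in sync with player name changes.
; BeginPlay creates the widget, adds it to the viewport and switches to UI-only input with a visible cursor.
; BindPlayerStates hooks the passed player state's name-change dispatcher and triggers an immediate list update.
; If the widget is not yet valid, the refresh retries on a short timer.
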(event `self.ReceiveBeginPlay`
  (bind _returnvalue (`GameplayStatics.GetPlayerController` 0))
  (bind _returnvalue_2 (`|CreateWidget` "/Game/ShootingGame/Widget/LobyWidget/LobbyHUDwidget.LobbyHUDwidget_C"))
  (bind _output_get (set `self.LobbyWidget` _returnvalue_2))
  (`UserWidget.AddToViewport` _output_get 0)
  (`WidgetBlueprintLibrary.SetInputMode_UIOnlyEx` _returnvalue null)
  (set `PlayerController.bShowMouseCursor` true _returnvalue))

(fn `BindPlayerStates`
  (params (PlayerStates :type "/Game/ShootingGame/GameMode/LobbyBP/BP_LobbyPlayerState Object Reference"))
  (add `/Game/ShootingGame/GameMode/LobbyBP/BP_LobbyPlayerState.NewEventDispatcher_ChangeName` PlayerStates (`|CreateDelegate` :!event `Event_ChangeName`))
  (`self.Event_ChangeName` ""))

(fn `Event_ChangeName`
  (params (NewName :type String))
  (`self.RF_ChangeName`))

(fn `RF_ChangeName`
  (bind _lobbywidget (`self.LobbyWidget`))
  (`/Engine/EditorBlueprintResources/StandardMacros.IsValid` _lobbywidget
    (:`Is Valid`
      (`/Game/ShootingGame/Widget/LobyWidget/LobbyHUDwidget.UpdatePlayerList` _lobbywidget))
    (:`Is Not Valid`
      (`KismetSystemLibrary.K2_SetTimer` null "RF_ChangeName" 0.1))))

(fn `UserConstructionScript`)