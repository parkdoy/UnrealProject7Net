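; BP_ShootingHud is the shooting game's HUD, creating the on-screen widget at BeginPlay and setting game-only input with the cursor hidden.
; It binds to HP and Armor dispatchers on BP_ShootingPlayerState, retrying on a short timer until the player state cast succeeds.
; Wrapper functions forward ammo, magazine, HP, armor and the position and visibility of a world-located F guide to the widget.
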(event `self.ReceiveBeginPlay`
  (bind _returnvalue (`GameplayStatics.GetPlayerController` 0))
  (bind _returnvalue_2 (`|CreateWidget` "/Game/ShootingGame/Widget/ShootingHudWidget.ShootingHudWidget_C"))
  (bind _output_get (set `self.HudWidget` _returnvalue_2))
  (`UserWidget.AddToViewport` _output_get 0)
  (`self.BindPlayerStats`)
  (`WidgetBlueprintLibrary.SetInputMode_GameOnly` _returnvalue)
  (set `PlayerController.bShowMouseCursor` false _returnvalue))

(fn `BindPlayerStats`
  (bind _asbp_shooting_player_state (cast `/Game/ShootingGame/GameMode/BP_ShootingPlayerState` (`Controller.PlayerState` (`GameplayStatics.GetPlayerController` 0)))
    (:`then`
      (add `/Game/ShootingGame/GameMode/BP_ShootingPlayerState.EventDispatcher_HP` _asbp_shooting_player_state (`|CreateDelegate` :!event `UpdateHP`))
      (add `/Game/ShootingGame/GameMode/BP_ShootingPlayerState.EventDispatcher_Armor` _asbp_shooting_player_state (`|CreateDelegate` :!event `UpdateArmor`)))
    (:`CastFailed`
      (`KismetSystemLibrary.K2_SetTimer` null "BindPlayerStats" 0.01))))

(fn `SetVisibilityGuideF`
  (params (InVisibility :type "ESlateVisibility Enum" :default "Visible"))
  (`/Game/ShootingGame/Widget/ShootingHudWidget.SetVisibilityGuideF` (`self.HudWidget`) InVisibility))

(fn `UpdateAmmo`
  (params (Ammo :type Integer))
  (`/Game/ShootingGame/Widget/ShootingHudWidget.SetAmmo` (`self.HudWidget`) Ammo))

(fn `UpdateArmor`
  (params (CurArmor :type "Float (double-precision)") (MaxArmor :type "Float (double-precision)"))
  (`/Game/ShootingGame/Widget/ShootingHudWidget.SetArmor` (`self.HudWidget`) CurArmor MaxArmor))

(fn `UpdateGuideF`
  (params (WorldLocation :type "Vector Structure"))
  (`/Game/ShootingGame/Widget/ShootingHudWidget.SetPositionGuideF` (`self.HudWidget`) WorldLocation))

(fn `UpdateHP`
  (params (CurHP :type "Float (double-precision)") (MaxHP :type "Float (double-precision)"))
  (`/Game/ShootingGame/Widget/ShootingHudWidget.SetHP` (`self.HudWidget`) CurHP MaxHP))

(fn `UpdateMag`
  (params (Mag :type Integer))
  (`/Game/ShootingGame/Widget/ShootingHudWidget.SetMag` (`self.HudWidget`) Mag))

(fn `UserConstructionScript`)