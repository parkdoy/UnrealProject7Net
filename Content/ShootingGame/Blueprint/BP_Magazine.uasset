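; BP_Magazine is a magazine pickup item for the shooting game that spins its static mesh every tick.
; Its UseItem override runs the parent check, then casts the user to BP_ShootingCharacter, calls AddMag and destroys the pickup.
; The event graph also holds disconnected leftovers: an authority-checked pickup path and a timed hide-and-reappear sequence that never run.
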(event `self.ReceiveTick`
  (params (DeltaSeconds :type "Float (single-precision)"))
  (`SceneComponent.K2_AddRelativeRotation` (`self.StaticMesh`) (struct :`Yaw` 2.0) false false))

(fn `UseItem`
  (params (Character :type "Character Object Reference"))
  (returns (IsUse :type Boolean))
  (bind _isuse (`parent.UseItem` Character))
  (if _isuse
    (bind _asbp_shooting_character (cast `/Game/ShootingGame/GameMode/BP_ShootingCharacter` Character))
    (`/Game/ShootingGame/GameMode/BP_ShootingCharacter.AddMag` _asbp_shooting_character)
    (`self.K2_DestroyActor`)))

(fn `UserConstructionScript`)