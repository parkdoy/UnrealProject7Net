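; BP_Medicine is a healing item for the shooting game that restores a fixed amount of health to the character that uses it.
; Its UseItem override calls the parent check first, and on success adds the heal through the character's BP_ShootingPlayerState, then destroys the actor.
; The EventGraph holds only empty events and disconnected leftover logic for an older authority-checked heal.
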(fn `UseItem`
  (params (Character :type "Character Object Reference"))
  (bind _isuse (`parent.UseItem` Character))
  (if _isuse
    (bind _asbp_shooting_player_state (cast `/Game/ShootingGame/GameMode/BP_ShootingPlayerState` (`Pawn.PlayerState` Character)))
    (`/Game/ShootingGame/GameMode/BP_ShootingPlayerState.AddHeal` _asbp_shooting_player_state 50.0)
    (`self.K2_DestroyActor`)))

(fn `UserConstructionScript`)